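; Deathmatch AI controller that runs BT_DeathMatch and seeds its blackboard with target index and AI state values on BeginPlay.
; Perception updates feed a sight handler that sets or clears the seen player.
; Any other sight update, including losing sight, changes AIState and requests a one-second prediction of that actor's position.
; A prediction handler stores the predicted player location as LoseSightLocation in the blackboard.
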(event OnTargetPerceptionUpdated(AIPerception)
  (params (Actor :type Actor%20Object%20Reference) (Stimulus :type AI%20Stimulus%20Structure))
  (CallFunction|AISenseSeeActor Actor Stimulus)
  (CallFunction|AIPrediction Actor Stimulus))

(event EventBeginPlay
  (AI|RunBehaviorTree "/Game/Blueprint/AI/BT_DeathMatch.BT_DeathMatch")
  (Class|BlackboardComponent|SetValueasInt (AI|GetBlackboard 0) (Utilities|Name|MakeLiteralName "TargetIndex"))
  (AI|Components|Blackboard|SetValueasBool (AI|GetBlackboard 0) (Utilities|Name|MakeLiteralName "TargetIndexAdd") true)
  (AI|Components|Blackboard|SetValueasEnum (AI|GetBlackboard 0) (Utilities|Name|MakeLiteralName "AIState")))

(fn ConstructionScript)

(fn AISenseSeeActor
  (params (Actor :type Actor%20Object%20Reference) (AIStimulus :type AI%20Stimulus%20Structure%20%28by%20ref%29))
  (bind _returnvalue (Utilities|Name|MakeLiteralName "SeePlayerActor"))
  (bind _returnvalue_2 (AI|GetBlackboard 0))
  (bind _returnvalue_3 (Utilities|Name|MakeLiteralName "SeePlayer"))
  (bind _returnvalue_4 (AI|GetBlackboard 0))
  (bind _returnvalue_5 (Class|AIPerceptionSystem|GetSenseClassforStimulus AIStimulus))
  (if (== _returnvalue_5 "/Script/AIModule.AISense_Sight")
    (if (and (Actor|ActorHasTag Actor "Player") (.bSuccessfullySensed (Utilities|Struct|BreakAIStimulus AIStimulus)))
      (AI|Components|Blackboard|SetValueasBool _returnvalue_4 _returnvalue_3 true)
      (AI|Components|Blackboard|SetValueasObject _returnvalue_2 _returnvalue Actor)
      (else
        (AI|Components|Blackboard|SetValueasBool _returnvalue_4 _returnvalue_3 false)
        (AI|Components|Blackboard|SetValueasObject _returnvalue_2 _returnvalue 0)
        (AI|Components|Blackboard|SetValueasEnum (AI|GetBlackboard 0) (Utilities|Name|MakeLiteralName "AIState") 1)
        (Class|AISensePrediction|RequestPawnPredictionEvent (Pawn|GetControlledPawn) Actor 1.0)))
    (return)
    (else
      (return))))

(fn AIPrediction
  (params (Actor :type Actor%20Object%20Reference) (AIStimulus :type AI%20Stimulus%20Structure%20%28by%20ref%29))
  (bind (_age _expirationage _strength _stimuluslocation _receiverlocation _tag _bsuccessfullysensed) (Utilities|Struct|BreakAIStimulus AIStimulus))
  (bind _returnvalue (Class|AIPerceptionSystem|GetSenseClassforStimulus AIStimulus))
  (if (== _returnvalue "/Script/AIModule.AISense_Prediction")
    (if (and (Actor|ActorHasTag Actor "Player") _bsuccessfullysensed)
      (AI|Components|Blackboard|SetValueasVector (AI|GetBlackboard 0) (Utilities|Name|MakeLiteralName "LoseSightLocation") _stimuluslocation)
      (return)
      (else
        (return)))
    (else
      (return))))
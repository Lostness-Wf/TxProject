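; BP_MainMenuController is a player controller that switches from an initial UI screen to the main menu on player input.
; Any touch event passes through a shared DoOnce, while Space Bar bypasses it and runs the same switch directly.
; If UIMain is valid, it is removed, a UI_MainMenu widget is added to the viewport, and input becomes UI-only.
; GetModuleName returns the controller's name, likely for script binding.
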(event Input|KeyboardEvents|SpaceBar
  (params (Key :type Key%20Structure :default "None"))
  (:Pressed
    (bind _ui_main (Variables|Default|GetUI_Main)
      (:then
        (Widget|RemovefromParent _ui_main)
        (bind _returnvalue (UserInterface|CreateWidget "/Game/Blueprint/UI/UI_MainMenu.UI_MainMenu_C" self))
        (bind _output_get (Variables|Default|SetUI_MainMenu _returnvalue))
        (UserInterface|Viewport|AddtoViewport _output_get 0)
        (Input|SetInputModeUIOnly self 0 "DoNotLock" false))
      (:else))))

(event Input|TouchEvents|InputTouch
  (params (Location :type Vector) (FingerIndex :type ETouchIndex%20Enum))
  (:Pressed
    (Utilities|FlowControl|DoOnce false :!label _label
      (:Completed
        (bind _ui_main (Variables|Default|GetUI_Main)
          (:then
            (Widget|RemovefromParent _ui_main)
            (bind _returnvalue (UserInterface|CreateWidget "/Game/Blueprint/UI/UI_MainMenu.UI_MainMenu_C" self))
            (bind _output_get (Variables|Default|SetUI_MainMenu _returnvalue))
            (UserInterface|Viewport|AddtoViewport _output_get 0)
            (Input|SetInputModeUIOnly self 0 "DoNotLock" false))
          (:else)))))
  (:Released
    (goto _label))
  (:Moved
    (goto _label)))

(fn ConstructionScript)

(fn GetModuleName
  (return "BP_MainMenuController"))
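; Deathmatch game mode that runs a timed round, spawns players and keeps score for a multiplayer FPS.
; The first login gathers PlayerStarts and starts a one-second countdown pushed to every controller, which ends the game for all at zero.
; Spawn requests create BP_Attacker characters, cycling through the starts round-robin.
; A controller-to-data map holds names and scores, lowered on death, raised on kills, then sent to all players.
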(event Custom|RequestSpawn
  (params (PlayerController :type BP%20Multi%20FPS%20Player%20Controller%20Object%20Reference))
  ;[1 1 1] 选择出生点
  (Default|SpawnPlayerCharacter PlayerController "/Game/Blueprint/Player/BP_Attacker.BP_Attacker_C" (Transformation|GetActorTransform (Utilities|Array|Get(acopy) (Variables|Default|GetCharacterSpawnPoints) (Variables|Default|GetSpawnIndex))))
  (Math|Integer|IncrementInt (Variables|Default|GetSpawnIndex)
    (:%20%20
      (if (>= (Variables|Default|GetSpawnIndex) (Utilities|Array|Length (Variables|Default|GetCharacterSpawnPoints)))
        (Variables|Default|SetSpawnIndex 0)))))

(event Custom|UpdateValues
  ;[1 1 1] 更新玩家信息
  (bind _keys (Utilities|Map|Keys (Variables|Default|GetPlayerGameDataMap)))
  (for _array_element _keys
    (bind _values (Utilities|Map|Values (Variables|Default|GetPlayerGameDataMap)))
    (Default|UpdateValues _array_element _values)))

(event Custom|OtherDeath
  (params (PlayerController :type BP%20Multi%20FPS%20Player%20Controller%20Object%20Reference))
  (bind _playergamedatamap (Variables|Default|GetPlayerGameDataMap))
  (bind _value (Utilities|Map|Find _playergamedatamap PlayerController))
  (bind (_playername _playerscore) (Utilities|Struct|BreakDeathMatchPlayerData _value))
  ;[1 1 1] 别人死亡
  (Variables|Default|SetKillPlayerName _playername)
  (Variables|Default|SetKillPlayerScore _playerscore)
  (Utilities|Map|Remove _playergamedatamap PlayerController)
  (Utilities|Map|Add (Variables|Default|GetPlayerGameDataMap) PlayerController (Utilities|Struct|MakeDeathMatchPlayerData (Variables|Default|GetKillPlayerName) (+ (Variables|Default|GetKillPlayerScore) 15)))
  (CallFunction|UpdateValues))

(event Custom|SelfDeath
  (params (PlayerController :type BP%20Multi%20FPS%20Player%20Controller%20Object%20Reference))
  (bind _playergamedatamap (Variables|Default|GetPlayerGameDataMap))
  (bind _value (Utilities|Map|Find _playergamedatamap PlayerController))
  (bind (_playername _playerscore) (Utilities|Struct|BreakDeathMatchPlayerData _value))
  ;[1 1 1] 自己死亡
  (Variables|Default|SetHitPlayerName _playername)
  (Variables|Default|SetHitPlayerScore _playerscore)
  (Utilities|Map|Remove _playergamedatamap PlayerController)
  (Utilities|Map|Add (Variables|Default|GetPlayerGameDataMap) PlayerController (Utilities|Struct|MakeDeathMatchPlayerData (Variables|Default|GetHitPlayerName) (- (Variables|Default|GetHitPlayerScore) 10)))
  (CallFunction|UpdateValues))

(event Custom|GameStateSet
  ;[1 1 1] 注释
  (bind _outactors (Actor|GetAllActorsOfClass "/Script/Engine.PlayerStart"))
  (Variables|Default|SetCharacterSpawnPoints _outactors)
  (bind _returnvalue (Utilities|Time|SetTimerbyEvent (delegate Custom|Doawn) 1.0 true))
  (Variables|Default|SetDownTimerHandle _returnvalue))

(event Custom|Doawn
  ;[1 1 1] 注释
  (Math|Integer|DecrementInt (Variables|Default|GetRoundTime)
    (:%20%20
      (bind _keys (Utilities|Map|Keys (Variables|Default|GetPlayerGameDataMap)))
      (for _array_element _keys
        (Default|ClientUpdateDownTime _array_element (Variables|Default|GetRoundTime))
        (if (<= (Variables|Default|GetRoundTime) 0)
          (Utilities|Time|ClearandInvalidateTimerbyHandle (Variables|Default|GetDownTimerHandle))
          (CallFunction|EndGame))))))

(event Custom|EndGame
  ;[1 1 1] 结束游戏
  (bind _keys (Utilities|Map|Keys (Variables|Default|GetPlayerGameDataMap)))
  (for _array_element _keys
    (Default|ClientEndGame _array_element)))

(event EventPostLogin
  (params (NewPlayer :type Player%20Controller%20Object%20Reference))
  ;[1 1 1] 玩家登录
  (if (Variables|Default|GetFirstCharacterJoin)
    _
    (else
      (CallFunction|GameStateSet)
      (Variables|Default|SetFirstCharacterJoin true)))
  (bind _asbp_multi_fpsplayer_controller (Utilities|Casting|CastToBP_MultiFPSPlayerController NewPlayer))
  (Default|StartSpawn _asbp_multi_fpsplayer_controller)
  (Utilities|Map|Add (Variables|Default|GetPlayerGameDataMap) _asbp_multi_fpsplayer_controller (Utilities|Struct|MakeDeathMatchPlayerData (Utilities|String|StringToName (Utilities|GetObjectName _asbp_multi_fpsplayer_controller)))))

(fn ConstructionScript)